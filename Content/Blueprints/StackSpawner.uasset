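; Spawner actor for a tile-stacking mechanic that builds a starting tower and slides a live tile for placement.
; BeginPlay stacks tiles by raising its own root after each spawn, then SpawnTile creates the current tile at the LeftSpawner component.
; Tick moves that tile along negative world X at a frame-rate-independent speed until PlaceTile clears CanMove, which does not spawn a replacement.
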(event Custom|SpawnTile
  (bind _returnvalue (Game|SpawnActorfromClass "/Game/Blueprints/Tile.Tile_C" (Math|Transform|MakeTransform (Transformation|GetWorldLocation (Variables|Default|GetLeftSpawner))) "Undefined" 0 0))
  (Variables|Default|SetCurrentTile _returnvalue)
  (Variables|Default|SetCanMove true))

(event Custom|Place%20Tile
  (Variables|Default|SetCanMove false))

(event EventBeginPlay
  (for _index (range 0 (Variables|Default|GetNumberOfTilesToSpawn))
    (Game|SpawnActorfromClass "/Game/Blueprints/Tile.Tile_C" (Transformation|GetWorldTransform (Variables|Default|GetDefaultSceneRoot)) "Undefined" 0 0)
    (Transformation|AddWorldOffset (Variables|Default|GetDefaultSceneRoot) (Math|Vector|MakeVector 0.0 0.0 (Variables|Default|GetZValueDistance)) false false))
  (CallFunction|SpawnTile))

(event Collision|EventActorBeginOverlap
  (params (OtherActor :type Actor%20Object%20Reference)))

(event EventTick
  (params (DeltaSeconds :type Float%20%28single-precision%29))
  (if (and (Variables|Default|GetCanMove) (Utilities|IsValid (Variables|Default|GetCurrentTile)))
    (CallFunction|MoveTile (Variables|Default|GetCurrentTile) DeltaSeconds (Variables|Default|GetTileSpeed))))

(fn ConstructionScript)

(fn MoveTile
  (params (CurrentTile :type Tile%20Object%20Reference) (DeltaTime :type Float%20%28single-precision%29) (Speed :type Float%20%28single-precision%29))
  (Transformation|AddActorWorldOffset CurrentTile (Math|Vector|MakeVector (* DeltaTime Speed -1.0) 0.0 0.0)))